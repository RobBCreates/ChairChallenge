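; Interactable chair for the Musical Throne challenge that seats one hero, either player or AI.
; Interacting with a free chair hides the popup, locks local player 0's movement and actions, and calls Sitdown.
; Sitdown flags the hero as sitting, disables its collision and gravity, teleports it to the Sit point, marks the chair occupied and fires OnChairOccupied.
; Interaction popups ignore AI heroes.
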(event EventBeginPlay)

(event Collision|EventActorBeginOverlap
  (params (OtherActor :type Actor%20Object%20Reference)))

(event EventTick
  (params (DeltaSeconds :type Float%20%28single-precision%29)))

(fn ConstructionScript)

(fn Sitdown
  (params (GMCHero :type GMC%20Hero%20Object%20Reference))
  (bind _output_get (Variables|Default|SetCurrentPlayer GMCHero))
  (bind _asbp_gmchero_003 (Utilities|Casting|CastToBP_GMCHero_003 _output_get)
    (:then
      (Variables|/Game/GMC/Challenges/Challenge_003_MusicalThrone/Blueprints/Characters/BP_GMCHero_003.BP_GMCHero_003_C|SetbSitting _asbp_gmchero_003 true))
    (:CastFailed
      (bind _asbp_gmchero_ai (Utilities|Casting|CastToBP_GMCHero_AI (Variables|Default|GetCurrentPlayer)))
      (Variables|/Game/GMC/Challenges/Challenge_003_MusicalThrone/Blueprints/Characters/BP_GMCHero_003.BP_GMCHero_003_C|SetbSitting _asbp_gmchero_ai true)))
  (CallFunction|AttachPlayer)
  (Variables|Default|SetCanInteract false)
  (Variables|Default|SetbOccupied true)
  (Default|CallOnChairOccupied)
  (Class|GMCChair|ResetGameplayTags))

(fn AttachPlayer
  (bind _sit (Variables|Default|GetSit))
  (bind _returnvalue (Transformation|GetWorldTransform _sit))
  (Collision|SetCollisionEnabled (Variables|/Script/Engine.Character|GetCapsuleComponent (Variables|Default|GetCurrentPlayer)) "NoCollision")
  (Variables|/Script/Engine.CharacterMovementComponent|SetGravityScale (Variables|/Script/Engine.Character|GetCharacterMovement (Variables|Default|GetCurrentPlayer)) 0.0)
  (Transformation|SetActorTransform (Variables|Default|GetCurrentPlayer) (Math|Transform|MakeTransform (.location _returnvalue) (.rotation _returnvalue) (Class|Actor|GetActorRelativeScale3D (Variables|Default|GetCurrentPlayer))) false true))

(fn DisplayInteractPopUp
  (params (Caller :type Actor%20Object%20Reference))
  (Utilities|Casting|CastToBP_GMCHero_AI Caller
    (:CastFailed
      (if (Variables|Default|GetCanInteract)
        (Class|GMCInteractableComponent|CallDisplayPopUp (Variables|Default|GetGMCInteractable))
        (return false)))))

(fn HideInteractPopUp
  (params (Caller :type Actor%20Object%20Reference))
  (Utilities|Casting|CastToBP_GMCHero_AI Caller
    (:CastFailed
      (Class|GMCInteractableComponent|CallHidePopUp (Variables|Default|GetGMCInteractable))
      (return false))))

(fn Interact
  (params (CallingActor :type Actor%20Object%20Reference))
  (if (not (Variables|Default|GetbOccupied))
    (CallFunction|HideInteractPopUp)
    (bind _asbp_gmcplayer_controller_003 (Utilities|Casting|CastToBP_GMCPlayerController_003 (Game|GetPlayerController 0)))
    (Class|GMCPlayerController|LockPlayerMovement _asbp_gmcplayer_controller_003 true)
    (Class|GMCPlayerController|LockPlayerActions _asbp_gmcplayer_controller_003 true)
    (CallFunction|HideInteractPopUp _asbp_gmcplayer_controller_003)
    (bind _asgmchero (Utilities|Casting|CastToGMCHero CallingActor))
    (CallFunction|Sitdown _asgmchero)
    (return 0)
    (else
      (return 0))))