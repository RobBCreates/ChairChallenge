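; AI-controlled hero for the Musical Throne challenge, colored as a red, blue or green knight by its team.
; Setup functions switch Blackboard flags on its AI controller between waiting, music playing and music stopped states.
; On the game mode's fade out, a loser is destroyed, while others teleport back to their starting transform and wait.
; Losing plays a defeat animation.
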(event Custom|OnLose
  (Components|Animation|PlayAnimation (Variables|Character|GetMesh) "/Game/GMC/Challenges/Challenge_003_MusicalThrone/Animations/Anim_Lose.Anim_Lose" false))

(event EventBeginPlay
  (Variables|Default|SetStartingPosition (Transformation|GetActorTransform))
  (bind _asbp_gmcgame_mode_003 (Utilities|Casting|CastToBP_GMCGameMode_003 (Game|GetGameMode)))
  (EventDispatchers|BindEventtoOnFadeOut _asbp_gmcgame_mode_003 (delegate EventOnFadeOut)))

(event EventOnFadeOut
  (|CallParentFunction)
  (if (Variables|Default|GetbIsLoser)
    (Actor|DestroyActor)
    (else
      (CallFunction|ResettoStarting))))

(fn ConstructionScript
  (CallFunction|SetTeamColor))

(fn SetupWaiting
  (bind _asbp_gmc_aicontroller (Utilities|Casting|CastToBP_GMC_AIController (AI|GetAIController self)))
  (bind _output_get (LocalVariables|SetBlackboard (AI|GetBlackboard _asbp_gmc_aicontroller)))
  (AI|Components|Blackboard|SetValueasBool _output_get (Utilities|Name|MakeLiteralName "IsWaiting") true)
  (AI|Components|Blackboard|SetValueasBool (LocalVariables|GetBlackboard) (Utilities|Name|MakeLiteralName "IsMusicPlaying") false))

(fn SetupMusicPlaying
  (bind _asbp_gmc_aicontroller (Utilities|Casting|CastToBP_GMC_AIController (AI|GetAIController self)))
  (bind _output_get (LocalVariables|SetBlackboard (AI|GetBlackboard _asbp_gmc_aicontroller)))
  (AI|Components|Blackboard|SetValueasBool _output_get (Utilities|Name|MakeLiteralName "IsWaiting") false)
  (AI|Components|Blackboard|SetValueasBool (LocalVariables|GetBlackboard) (Utilities|Name|MakeLiteralName "IsMusicPlaying") true))

(fn SetupMusicStopped
  (bind _asbp_gmc_aicontroller (Utilities|Casting|CastToBP_GMC_AIController (AI|GetAIController self)))
  (bind _output_get (LocalVariables|SetBlackboard (AI|GetBlackboard _asbp_gmc_aicontroller)))
  (AI|Components|Blackboard|SetValueasBool _output_get (Utilities|Name|MakeLiteralName "IsWaiting") false)
  (AI|Components|Blackboard|SetValueasBool (LocalVariables|GetBlackboard) (Utilities|Name|MakeLiteralName "IsMusicPlaying") false)
  (AI|Components|Blackboard|SetValueasBool (LocalVariables|GetBlackboard) (Utilities|Name|MakeLiteralName "IsMusicStopped") true))

(fn ResettoStarting
  (bind _startingposition (Variables|Default|GetStartingPosition))
  (Transformation|SetActorTransform (Math|Transform|MakeTransform (.location _startingposition) (.rotation _startingposition) "1,1,1") false true)
  (CallFunction|SetupWaiting))

(fn SetTeamColor
  (bind _mesh (Variables|Character|GetMesh))
  (switch Utilities|FlowControl|Switch|SwitchonETeamColor (Variables|Default|GetTeamColor)
    (:NewEnumerator0
      (Rendering|Material|SetMaterial _mesh 0 (Variables|Default|GetRedKnight)))
    (:NewEnumerator1
      (Rendering|Material|SetMaterial _mesh 0 (Variables|Default|GetBlueKnight)))
    (:NewEnumerator2
      (Rendering|Material|SetMaterial _mesh 0 (Variables|Default|GetGreenKnight)))))