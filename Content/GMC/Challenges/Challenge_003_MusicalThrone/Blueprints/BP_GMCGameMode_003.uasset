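; Game mode for the Musical Throne challenge, a musical-chairs game pitting the player against AI heroes over several rounds.
; Rounds run from screen fade and countdown into music that stops on a random timer, switching AI state and firing event dispatchers.
; When chairs fill, a standing AI is eliminated before the next round.
; A standing player loses to an AI, while outlasting all rounds makes the player the winner.
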(event Custom|GameOver
  (params (Winner :type Actor%20Object%20Reference))
  (Variables|Default|SetbGameOver true)
  (CallFunction|FadeOut)
  (Utilities|FlowControl|Delay (Variables|Default|GetFadeTime))
  (bind _ascharacter (Utilities|Casting|CastToCharacter Winner))
  (Default|CallOnGameOver _ascharacter)
  (Utilities|FlowControl|Delay 0.2)
  (CallFunction|Fadein)
  (bind _returnvalue (Audio|CreateSound2D "/Game/GMC/Challenges/Challenge_003_MusicalThrone/Audio/WinningCelebration.WinningCelebration" 1.0 1.0 0.0 0))
  (Audio|Components|Audio|FadeIn _returnvalue 0.5 1.0 0.0 "Linear" :!class /Script/Engine.AudioComponent))

(event Custom|StartCountdown
  (bind _countdowntimestart (Variables|Default|GetCountdownTimeStart))
  (CallFunction|FadeOut)
  (Utilities|FlowControl|Delay (Variables|Default|GetFadeTime))
  (Default|CallOnFadeOut)
  (Utilities|FlowControl|Delay 0.2)
  (CallFunction|Fadein)
  (Audio|PlaySound2D "/Game/GMC/Challenges/Challenge_003_MusicalThrone/Audio/trumpet-brass-fanfare.trumpet-brass-fanfare" 1.0 1.0 0.0 0 0)
  (Utilities|FlowControl|Delay (Variables|Default|GetFadeTime))
  (Default|CallOnCountdownStarted _countdowntimestart)
  (Variables|Default|SetCountdownTimeRemaining _countdowntimestart)
  (Utilities|FlowControl|Delay 1.0)
  (CallFunction|TickCountdown))

(event Custom|StartGame
  (Variables|Default|SetbGameOver false)
  (Default|CallOnGameStarted)
  (CallFunction|StartMusic))

(event Custom|StartMusic
  (Variables|Default|SetbMusicPaused false)
  (if (not (Variables|Default|GetbGameOver))
    (Default|CallOnStartMusic)
    (Utilities|FlowControl|Delay 0.6)
    (CallFunction|PlayMusic)
    (bind _outactors (Actor|GetAllActorsOfClass "/Game/GMC/Challenges/Challenge_003_MusicalThrone/Blueprints/Characters/BP_GMCHero_AI.BP_GMCHero_AI_C"))
    (for _array_element _outactors
      (Default|SetupMusicPlaying _array_element)
      (Utilities|Time|SetTimerbyEvent (delegate Custom|StopMusic) (Math|Random|RandomFloatinRange 5.0 1e+01)))))

(event Custom|StopMusic
  (Variables|Default|SetbMusicPaused true)
  (Default|CallOnStopMusic)
  (CallFunction|PauseMusic)
  (bind _outactors (Actor|GetAllActorsOfClass "/Game/GMC/Challenges/Challenge_003_MusicalThrone/Blueprints/Characters/BP_GMCHero_AI.BP_GMCHero_AI_C"))
  (for _array_element _outactors
    (Default|SetupMusicStopped _array_element)))

(event Custom|AllChairsOccupied
  (bind _ai_players (Variables|Default|GetAI_Players))
  (CallFunction|CheckSitting)
  (bind _asbp_gmchero_ai (Utilities|Casting|CastToBP_GMCHero_AI (Variables|Default|GetLoser))
    (:then
      (Default|OnLose _asbp_gmchero_ai)
      (Variables|/Game/GMC/Challenges/Challenge_003_MusicalThrone/Blueprints/Characters/BP_GMCHero_AI.BP_GMCHero_AI_C|SetbIsLoser _asbp_gmchero_ai true)
      (Utilities|Array|RemoveItem (Variables|Default|GetAI_Players) _asbp_gmchero_ai)
      (Utilities|FlowControl|Delay 3.0)
      (CallFunction|NextRound))
    (:CastFailed
      (CallFunction|GameOver (Utilities|Array|Get(acopy) _ai_players (Math|Random|RandomInteger (- (Utilities|Array|Length _ai_players) 1)))))))

(event EventBeginPlay
  (CallFunction|SetupGame))

(fn ConstructionScript)

(fn SetupGame
  (bind _returnvalue (Game|GetPlayerController 0))
  (bind _returnvalue_2 (Audio|SpawnSound2D "/Game/GMC/Challenges/Challenge_003_MusicalThrone/Audio/MusicalChairs.MusicalChairs" 1.0 1.0 0.0 0))
  (Variables|Default|SetMusic _returnvalue_2)
  (bind _returnvalue_3 (UserInterface|CreateWidget "/Game/GMC/Challenges/Challenge_003_MusicalThrone/UI/WBP_HUD_003.WBP_HUD_003_C" _returnvalue))
  (UserInterface|Viewport|AddtoViewport _returnvalue_3 0)
  (Input|SetInputModeGameOnly _returnvalue)
  (Variables|/Script/Engine.PlayerController|SetbShowMouseCursor _returnvalue false)
  (CallFunction|GetPlayers))

(fn RunGame
  (if (not (Variables|Default|GetbGameOver))
    _))

(fn NextRound
  (if (not (Variables|Default|GetbGameOver))
    (bind _result (Math|Integer|IncrementInt (Variables|Default|GetCurrentRound))
      (:%20%20
        (if (> _result (Variables|Default|GetMaxRounds))
          (CallFunction|GameOver (Variables|Default|GetPlayerCharacter))
          (else
            (CallFunction|StartCountdown)))))))

(fn PauseMusic
  (Class|AudioComponent|SetPaused (Variables|Default|GetMusic) true)
  (Variables|Default|SetbMusicPaused true))

(fn PlayMusic
  (Utilities|IsValid (Variables|Default|GetMusic)
    (:Is%20Valid
      (Class|AudioComponent|SetPaused (Variables|Default|GetMusic) false)
      (Variables|Default|SetbMusicPaused false))
    (:Is%20Not%20Valid
      (bind _returnvalue (Audio|SpawnSound2D "/Game/GMC/Challenges/Challenge_003_MusicalThrone/Audio/MusicalChairs.MusicalChairs" 1.0 1.0 0.0 0))
      (bind _output_get (Variables|Default|SetMusic _returnvalue))
      (Audio|Components|Audio|Play _output_get 0.0))))

(fn FadeOut
  (bind _returnvalue (UserInterface|CreateWidget "/Game/GMC/Challenges/Challenge_003_MusicalThrone/UI/WBP_ScreenFade.WBP_ScreenFade_C" (Game|GetPlayerController 0)))
  (bind _output_get (Variables|Default|SetFadeScreen _returnvalue))
  (UserInterface|Viewport|AddtoViewport _output_get 0)
  (Variables|Default|SetFadeTime (Class|WidgetAnimation|GetEndTime (Variables|/Game/GMC/Challenges/Challenge_003_MusicalThrone/UI/WBP_ScreenFade.WBP_ScreenFade_C|GetFadeInOut _output_get)))
  (UserInterface|Animation|PlayAnimation _output_get (Variables|/Game/GMC/Challenges/Challenge_003_MusicalThrone/UI/WBP_ScreenFade.WBP_ScreenFade_C|GetFadeInOut _output_get) 0.0 1 "Forward" 1.0 false)
  (if (not (Variables|Default|GetbMusicPaused))
    (Audio|Components|Audio|FadeOut (Variables|Default|GetMusic) (Variables|Default|GetFadeTime) 0.0 "Linear" :!class /Script/Engine.AudioComponent)))

(fn Fadein
  (bind _fadescreen (Variables|Default|GetFadeScreen))
  (Utilities|IsValid _fadescreen
    (:Is%20Valid
      (UserInterface|Animation|PlayAnimation _fadescreen (Variables|/Game/GMC/Challenges/Challenge_003_MusicalThrone/UI/WBP_ScreenFade.WBP_ScreenFade_C|GetFadeInIn _fadescreen) 0.0 1 "Forward" 1.0 false))))

(fn ResetPlayer)

(fn TickCountdown
  (bind _result (Math|Float|DecrementFloat (Variables|Default|GetCountdownTimeRemaining))
    (:%20%20
      (if (> _result 0.0)
        (Utilities|Time|SetTimerbyFunctionName 0 "Tick Countdown" 1.0)
        (Default|CallOnTimerUpdated (Variables|Default|GetCountdownTimeRemaining))
        (Audio|PlaySound2D "/Game/GMC/Challenges/Challenge_003_MusicalThrone/Audio/low_snare.low_snare" 1.0 1.0 0.0 0 0)
        (else
          (CallFunction|StartGame)
          (Default|CallOnGameStarted))))))

(fn OnChairOccupied
  (bind _playerstartposition (Variables|Default|GetPlayerStartPosition))
  (bind _result (Math|Integer|DecrementInt (Variables|Default|GetNumOpenChairs))
    (:%20%20
      (if (== _result 0)
        (bind _asbp_gmchero_003 (Utilities|Casting|CastToBP_GMCHero_003 (Game|Player|GetPlayerPawn 0)))
        (bind _output_get (LocalVariables|SetCurrentPlayer _asbp_gmchero_003))
        (if (Variables|/Game/GMC/Challenges/Challenge_003_MusicalThrone/Blueprints/Characters/BP_GMCHero_003.BP_GMCHero_003_C|GetbSitting _output_get)
          (if (== (+ (Variables|Default|GetCurrentRound) 1) (Variables|Default|GetMaxRounds))
            (CallFunction|GameOver)
            (else
              (CallFunction|NextRound)
              (bind _outactors (Actor|GetAllActorsOfClass "/Game/GMC/Challenges/Challenge_003_MusicalThrone/Blueprints/Characters/BP_GMCHero_AI.BP_GMCHero_AI_C"))
              (bind _array_element (Utilities|Array|ForEachLoopwithBreak _outactors :!label _label)
                (:LoopBody
                  (if (not (Variables|/Game/GMC/Challenges/Challenge_003_MusicalThrone/Blueprints/Characters/BP_GMCHero_003.BP_GMCHero_003_C|GetbSitting _array_element))
                    (Actor|DestroyActor)
                    (goto _label Break)))
                (:Completed
                  (bind _outactors_2 (Actor|GetAllActorsOfClass "/Game/GMC/Challenges/Challenge_003_MusicalThrone/Blueprints/BP_StartingPlatform.BP_StartingPlatform_C"))
                  (for _array_element_2 _outactors_2
                    (LocalVariables|SetCurrentPlatform _array_element_2)
                    (if (Utilities|IsValid (Variables|/Game/GMC/Challenges/Challenge_003_MusicalThrone/Blueprints/BP_StartingPlatform.BP_StartingPlatform_C|GetCharacter _array_element_2))
                      (Default|PlaceCharactersinPosition (LocalVariables|GetCurrentPlatform))))
                  (bind _asbp_gmchero_003_2 (Utilities|Casting|CastToBP_GMCHero_003 (Game|Player|GetPlayerPawn 0)))
                  (Transformation|Teleport _asbp_gmchero_003_2 (.location _playerstartposition) (.rotation _playerstartposition))
                  (Variables|/Game/GMC/Challenges/Challenge_003_MusicalThrone/Blueprints/Characters/BP_GMCHero_003.BP_GMCHero_003_C|SetbSitting _asbp_gmchero_003_2 false)))))
          (else
            ;[1 1 1] player lost
            (bind _outactors_3 (Actor|GetAllActorsOfClass "/Game/GMC/Challenges/Challenge_003_MusicalThrone/Blueprints/Characters/BP_GMCHero_AI.BP_GMCHero_AI_C"))
            (CallFunction|GameOver (Utilities|Array|Get(acopy) _outactors_3))))))))

(fn PrepareRound
  ;[1 1 1] fade out teleport player and ai that are still valid
)

(fn GetPlayers
  (bind _asbp_gmchero_003 (Utilities|Casting|CastToBP_GMCHero_003 (Game|Player|GetPlayerPawn 0)))
  (Variables|Default|SetPlayerCharacter _asbp_gmchero_003)
  (bind _outactors (Actor|GetAllActorsOfClass "/Game/GMC/Challenges/Challenge_003_MusicalThrone/Blueprints/Characters/BP_GMCHero_AI.BP_GMCHero_AI_C"))
  (for _array_element _outactors
    (Utilities|Array|AddUnique (Variables|Default|GetAI_Players) _array_element)))

(fn CheckSitting
  (bind _playercharacter (Variables|Default|GetPlayerCharacter))
  (Default|HideInteractPopUp _playercharacter)
  (if (Variables|/Game/GMC/Challenges/Challenge_003_MusicalThrone/Blueprints/Characters/BP_GMCHero_003.BP_GMCHero_003_C|GetbSitting _playercharacter)
    (for _array_element (Variables|Default|GetAI_Players)
      (bind _output_get (LocalVariables|SetCurrentAI _array_element))
      (if (not (Variables|/Game/GMC/Challenges/Challenge_003_MusicalThrone/Blueprints/Characters/BP_GMCHero_003.BP_GMCHero_003_C|GetbSitting _output_get))
        (Variables|Default|SetLoser (LocalVariables|GetCurrentAI))))
    (else
      (Variables|Default|SetLoser (Variables|Default|GetPlayerCharacter)))))