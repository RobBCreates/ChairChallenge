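; Rotating chair platform for the Musical Throne challenge, driven by BP_GMCGameMode_003 music and fade events.
; On fade-out it respawns seats from child component transforms: all chairs in round 1, one random fewer in round 2, only the throne in round 3.
; Music toggles an eased, timer-driven base spin and a timeline-animated wall with sound.
; Seat occupancy is counted, and the game mode is notified when every seat is taken.
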(event Custom|OnChairOccupied
  (bind _result (Math|Integer|IncrementInt (Variables|Default|GetOccupiedChairs))
    (:%20%20
      (if (== _result (Utilities|Array|Length (Variables|Default|GetActiveChairs)))
        (Default|AllChairsOccupied (Variables|Default|GetGameMode_003))))))

(event Custom|OnGameOver
  (params (WinningPlayer :type Character%20Object%20Reference)))

(event Custom|ToggleSpin
  (params (ShouldSpin :type Boolean))
  (if ShouldSpin
    (Variables|Default|SetbIsSpinning true)
    (bind _rotationmultiplier (Timeline|SpinEase PlayFromStart)
      (:Update
        (CallFunction|RotateBase (* _rotationmultiplier (Variables|Default|GetRotationAmount))))
      (:Finished
        (CallFunction|Spin)))
    (else
      (Variables|Default|SetbIsSpinning false)
      (Timeline|SpinEase ReverseFromEnd))))

(event Custom|AnimateWall
  (params (AnimateDown :type Boolean))
  (Audio|PlaySoundatLocation "/Game/GMC/Challenges/Challenge_003_MusicalThrone/Audio/heavy-stone-push.heavy-stone-push" (Transformation|GetWorldLocation (Variables|Default|GetWall)) "0, 0, 0" 0.5 1.0 0.0 0 0 0)
  (if AnimateDown
    (bind _zposition (Timeline|WallAnimation PlayFromStart)
      (:Update
        (Transformation|SetRelativeLocation (Variables|Default|GetWall) (Math|Vector|MakeVector 0.0 0.0 _zposition) false false)))
    (else
      (Timeline|WallAnimation ReverseFromEnd))))

(event Custom|OnGameStarted)

(event Custom|OnStartMusic
  (CallFunction|AnimateWall false)
  (Utilities|FlowControl|Delay 0.6)
  (CallFunction|ToggleSpin true))

(event Custom|OnStopMusic
  (Variables|Default|SetOccupiedChairs 0)
  (CallFunction|ToggleSpin false)
  (CallFunction|AnimateWall true))

(event Custom|OnFadeOut
  (CallFunction|DestroyChairs)
  (CallFunction|SetupSpawnPoints)
  (CallFunction|SpawnChairs))

(event EventBeginPlay
  (bind _asbp_gmcgame_mode_003 (Utilities|Casting|CastToBP_GMCGameMode_003 (Game|GetGameMode)))
  (Variables|Default|SetGameMode_003 _asbp_gmcgame_mode_003)
  (CallFunction|SetupBindings))

(fn ConstructionScript)

(fn RotateBase
  (params (RotationAmount :type Float%20%28single-precision%29))
  (bind _base (Variables|Default|GetBase))
  (bind _relativerotation (Variables|/Script/Engine.SceneComponent|GetRelativeRotation _base))
  (Transformation|SetRelativeRotation (Variables|Default|GetBase) (Math|Rotator|MakeRotator (.roll _relativerotation) (.pitch _relativerotation) (+ (.yaw _relativerotation) RotationAmount)) false false))

(fn Spin
  (if (Variables|Default|GetbIsSpinning)
    (CallFunction|RotateBase (Variables|Default|GetRotationAmount))
    (Utilities|Time|SetTimerbyFunctionName 0 "Spin" (Variables|Default|GetSpinSpeed))))

(fn SetupBindings
  (bind _gamemode_003 (Variables|Default|GetGameMode_003))
  (EventDispatchers|BindEventtoOnGameStarted _gamemode_003 (EventDispatchers|CreateEvent :!event Custom|OnGameStarted))
  (EventDispatchers|BindEventtoOnGameOver _gamemode_003 (EventDispatchers|CreateEvent :!event Custom|OnGameOver))
  (EventDispatchers|BindEventtoOnStartMusic _gamemode_003 (EventDispatchers|CreateEvent :!event Custom|OnStartMusic))
  (EventDispatchers|BindEventtoOnStopMusic _gamemode_003 (EventDispatchers|CreateEvent :!event Custom|OnStopMusic))
  (EventDispatchers|BindEventtoOnFadeOut _gamemode_003 (EventDispatchers|CreateEvent :!event Custom|OnFadeOut)))

(fn SpawnChairs
  (bind _gamemode_003 (Variables|Default|GetGameMode_003))
  (bind _currentround (Variables|/Game/GMC/Challenges/Challenge_003_MusicalThrone/Blueprints/BP_GMCGameMode_003.BP_GMCGameMode_003_C|GetCurrentRound _gamemode_003))
  (if (< _currentround 4)
    (Utilities|FlowControl|Sequence
      (:then_0
        (switch int _currentround
          (:1
            (for _array_element (Variables|Default|GetChairSpawnPoints) :!label _label
              (bind _returnvalue (Game|SpawnActorfromClass "/Game/GMC/Challenges/Challenge_003_MusicalThrone/Blueprints/BP_Chair.BP_Chair_C" _array_element "Undefined" 0 0))
              (EventDispatchers|BindEventtoOnChairOccupied _returnvalue (EventDispatchers|CreateEvent :!event Custom|OnChairOccupied))
              (Utilities|Array|Add (Variables|Default|GetActiveChairs) _returnvalue)))
          (:2
            (CallFunction|RemoveRandomChair)
            (goto _label))
          (:3
            ;[1 1 1] throne
            (bind _returnvalue_2 (Game|SpawnActorfromClass "/Game/GMC/Challenges/Challenge_003_MusicalThrone/Blueprints/BP_Throne.BP_Throne_C" (Transformation|GetWorldTransform (Variables|Default|GetThrone)) "Undefined" 0 0))
            (EventDispatchers|BindEventtoOnChairOccupied _returnvalue_2 (EventDispatchers|CreateEvent :!event Custom|OnChairOccupied))
            (Utilities|Array|Add (Variables|Default|GetActiveChairs) _returnvalue_2))))
      (:then_1
        (for _array_element_2 (Variables|Default|GetActiveChairs)
          (Transformation|AttachComponentToComponent _array_element_2 (Variables|Default|GetChairs) "None" "KeepWorld" "KeepWorld" "KeepWorld" true))))))

(fn DestroyChairs
  (bind _activechairs (Variables|Default|GetActiveChairs))
  (if (> (Utilities|Array|Length _activechairs) 0)
    (for _array_element _activechairs
      (Actor|DestroyActor _array_element))
    (Utilities|Array|Clear (Variables|Default|GetActiveChairs))))

(fn SetupSpawnPoints
  (Utilities|Array|Clear (Variables|Default|GetChairSpawnPoints))
  (for _array_element (Components|GetChildrenComponents (Variables|Default|GetChairs) false)
    (Utilities|Array|AddUnique (Variables|Default|GetChairSpawnPoints) (Transformation|GetWorldTransform _array_element))))

(fn RemoveRandomChair
  (bind _chairspawnpoints (Variables|Default|GetChairSpawnPoints))
  (Utilities|Array|RemoveItem (Variables|Default|GetChairSpawnPoints) (Utilities|Array|Get(acopy) _chairspawnpoints (Math|Random|RandomIntegerinRange 0 (- (Utilities|Array|Length _chairspawnpoints) 1)))))