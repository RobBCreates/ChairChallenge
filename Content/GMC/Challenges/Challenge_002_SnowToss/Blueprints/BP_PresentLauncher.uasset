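; BP_PresentLauncher is an actor in the SnowToss challenge that launches random toys into the air.
; LaunchToy calls SpawnToy, which spawns a toy from a random DT_ToyList row if none exists, then applies a randomized upward velocity-change impulse and plays a sound.
; The launcher keeps one toy at a time and destroys it on overlap, such as when it falls back.
; Nothing in this Blueprint calls LaunchToy.
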(event EventBeginPlay)

(event Collision|EventActorBeginOverlap
  (params (OtherActor :type Actor%20Object%20Reference))
  (if (== OtherActor (Variables|Default|GetCurrentToy))
    (Actor|DestroyActor (Variables|Default|GetCurrentToy))))

(fn ConstructionScript)

(fn LaunchToy
  (CallFunction|SpawnToy)
  (Physics|AddImpulse (Variables|/Game/GMC/Challenges/Challenge_002_SnowToss/Blueprints/Toys/BP_Toy.BP_Toy_C|GetToyMesh (Variables|Default|GetCurrentToy)) (Math|Vector|MakeVector 0.0 0.0 (Math|Random|RandomFloatinRange 8e+02 9e+02)) "None" true)
  (Audio|PlaySoundatLocation "/Game/GMC/Challenges/Challenge_002_SnowToss/Audio/SFX/ToyLaunchQue.ToyLaunchQue" (Transformation|GetActorLocation) "0, 0, 0" 1.0 1.0 0.0 0 0 0))

(fn GetRandomToy
  (bind _outrownames (DataTable|GetDataTableRowNames "/Game/GMC/Challenges/Challenge_002_SnowToss/Data/DT_ToyList.DT_ToyList"))
  (bind _returnvalue (Utilities|GetDataTableRow "/Game/GMC/Challenges/Challenge_002_SnowToss/Data/DT_ToyList.DT_ToyList" (.OutItem (Utilities|Array|Random _outrownames)))
    (:then
      (return _returnvalue))))

(fn SpawnToy
  (Utilities|IsValid (Variables|Default|GetCurrentToy)
    (:Is%20Not%20Valid
      (bind _output_get (LocalVariables|SetToyData (CallFunction|GetRandomToy)))
      (bind _returnvalue (Game|SpawnActorfromClass (.toyclass _output_get) (Math|Transform|MakeTransform (Transformation|GetWorldLocation (Variables|Default|GetLaunchLocation)) "0,180.000000, 0" (* "1.000000,1.000000,1.000000" (.spawnscale (LocalVariables|GetToyData)))) "Undefined" self (LocalVariables|GetToyData) 0))
      (Variables|Default|SetCurrentToy _returnvalue))))