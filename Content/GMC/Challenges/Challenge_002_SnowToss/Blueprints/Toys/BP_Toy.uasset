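; BP_Toy is a target toy in the Snow Toss challenge that awards points when hit.
; On overlap with a BP_Snowball, it calls the snowball's OnHit, reports its ToyData to BP_GMCGameMode_002 and animates a points widget at its projected screen position.
; Interact also reports the hit, without the widget, and is the only path here that sets the Hit guard checked by both.
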(event EventBeginPlay)

(event Collision|EventActorBeginOverlap
  (params (OtherActor :type Actor%20Object%20Reference))
  (bind _toydata (Variables|Default|GetToyData))
  (if (not (Variables|Default|GetHit))
    (bind _asbp_snowball (Utilities|Casting|CastToBP_Snowball OtherActor))
    (Default|OnHit _asbp_snowball)
    (bind _asbp_gmcgame_mode_002 (Utilities|Casting|CastToBP_GMCGameMode_002 (Game|GetGameMode)))
    (Default|OnToyHit _asbp_gmcgame_mode_002 _toydata)
    (bind _returnvalue (UserInterface|CreateWidget "/Game/GMC/Challenges/Challenge_002_SnowToss/UI/WBP_002_HitPoints.WBP_002_HitPoints_C" (Game|GetPlayerController 0) (.ToyPoints (Utilities|Struct|BreakFToyData _toydata))))
    (Class|UserWidget|SetPositioninViewport _returnvalue (.ScreenLocation (Class|PlayerController|ProjectWorldLocationtoScreen (Game|GetPlayerController 0) (Transformation|GetActorLocation) false)) true)
    (UserInterface|Viewport|AddtoViewport _returnvalue 0)
    (Default|Animate _returnvalue)))

(fn ConstructionScript)

(fn DisplayInteractPopUp
  (return false))

(fn HideInteractPopUp
  (return false))

(fn Interact
  (params (CallingActor :type Actor%20Object%20Reference))
  (if (not (Variables|Default|GetHit))
    (bind _asbp_gmcgame_mode_002 (Utilities|Casting|CastToBP_GMCGameMode_002 (Game|GetGameMode)))
    (Default|OnToyHit _asbp_gmcgame_mode_002 (Variables|Default|GetToyData))
    (Variables|Default|SetHit true)
    (return 0)))