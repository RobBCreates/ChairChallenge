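; Player controller for the Snow Toss challenge (GMC Challenge 002) that turns attack requests into thrown snowballs.
; RequestAttack proceeds only once the game mode reports the game started and the current action status is not Attacking, then runs the parent attack logic.
; It spawns a BP_Snowball at the hero's SnowballSpawnLoc, stores it, and tosses it along the follow camera's forward vector.
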(event EventBeginPlay
  (|CallParentFunction) ; This node is disabled and will not be called.\nDrag off pins to build functionality.
)

(event EventTick
  (params (DeltaSeconds :type Float%20%28single-precision%29))
  (|CallParentFunction DeltaSeconds) ; This node is disabled and will not be called.\nDrag off pins to build functionality.
)

(event EventRequestAttack
  (bind _asbp_gmcgame_mode_002 (Utilities|Casting|CastToBP_GMCGameMode_002 (Game|GetGameMode)))
  (if (and (Variables|/Game/GMC/Challenges/Challenge_002_SnowToss/Blueprints/BP_GMCGameMode_002.BP_GMCGameMode_002_C|GetGameStarted _asbp_gmcgame_mode_002) (Utilities|Enum|NotEqual(Enum) (Class|GMCPlayerController|GetActionStatus) "Attacking"))
    (|CallParentFunction)
    (bind _asbp_gmchero_002 (Utilities|Casting|CastToBP_GMCHero_002 (Game|Player|GetPlayerPawn 0)))
    (bind _returnvalue (Game|SpawnActorfromClass "/Game/GMC/Challenges/Challenge_002_SnowToss/Blueprints/BP_Snowball.BP_Snowball_C" (Transformation|GetWorldTransform (Variables|/Game/GMC/Challenges/Challenge_002_SnowToss/Blueprints/BP_GMCHero_002.BP_GMCHero_002_C|GetSnowballSpawnLoc _asbp_gmchero_002)) "AlwaysSpawn" self _asbp_gmchero_002))
    (bind _output_get (Variables|Default|SetSnowball _returnvalue))
    (Default|Toss _output_get (Math|Vector|GetForwardVector (Variables|/Script/GMChallenge.GMCHero|GetFollowCamera _asbp_gmchero_002)))))

(fn ConstructionScript
  (|CallParentFunction))