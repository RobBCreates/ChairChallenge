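; Game mode for the Snow Toss challenge, where launchers fire toys and hits earn points.
; HUD events start a looping timer that fires random launchers and later end the game, triggering the hero's third-person celebration and hit-toy stats.
; Toy hits record the toy, add its points and play a sound.
; Launcher selection recurses to avoid repeats, but re-evaluates Random at each use, so repeats remain possible.
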(event Custom|StartGame
  (Class|GMCGameMode|ShowHUD)
  (Variables|Default|SetGameStarted true)
  (bind _aswbp_002_hud (Utilities|Casting|CastToWBP_002_HUD (Class|GMCGameMode|GetHUD)))
  (bind _output_get (Variables|Default|SetHUD _aswbp_002_hud))
  (EventDispatchers|BindEventtoBeginLaunch _output_get (delegate Custom|BeginLaunch))
  (EventDispatchers|BindEventtoGameOver (Variables|Default|GetHUD) (delegate Custom|EndGame))
  (Default|StartCountdown (Variables|Default|GetHUD)))

(event Custom|EndGame
  (Variables|Default|SetGameOver true)
  (Utilities|Time|ClearTimerbyFunctionName 0 "FireRandomLauncher")
  (bind _asbp_gmchero_002 (Utilities|Casting|CastToBP_GMCHero_002 (Game|Player|GetPlayerPawn 0)))
  (Default|SwitchtoThirdPerson _asbp_gmchero_002)
  (Transformation|SetActorRotation _asbp_gmchero_002 "0,-90.000000, 0")
  (Default|Celebrate _asbp_gmchero_002)
  (bind _aswbp_002_hud (Utilities|Casting|CastToWBP_002_HUD (Class|GMCGameMode|GetHUD)))
  (Default|DisplayStats _aswbp_002_hud (Variables|Default|GetHitToys)))

(event Custom|BeginLaunch
  (Utilities|Time|SetTimerbyFunctionName 0 "FireRandomLauncher" 3.0 true))

(event Custom|OnToyHit
  (params (HitToy :type F%20Toy%20Data%20Structure))
  (Utilities|Array|Add (Variables|Default|GetHitToys) HitToy)
  (Variables|Default|SetTotalPoints (+ (Variables|Default|GetTotalPoints) (.ToyPoints (Utilities|Struct|BreakFToyData HitToy))))
  (Audio|PlaySound2D "/Game/GMC/Challenges/Challenge_002_SnowToss/Audio/UI/Special_Powerup_01_wav.Special_Powerup_01_wav" 1.0 1.0 0.0 0 0))

(event EventBeginPlay
  (bind _outactors (Actor|GetAllActorsOfClass "/Game/GMC/Challenges/Challenge_002_SnowToss/Blueprints/BP_PresentLauncher.BP_PresentLauncher_C"))
  (Variables|Default|SetPresentLaunchers _outactors))

(fn ConstructionScript)

(fn FireRandomLauncher
  (bind _presentlaunchers (Variables|Default|GetPresentLaunchers))
  (bind _outitem (Utilities|Array|Random _presentlaunchers))
  (if (not (Variables|Default|GetGameOver))
    (Utilities|IsValid _outitem
      (:Is%20Valid
        (if (!= (Variables|Default|GetActiveLauncher) _outitem)
          (bind _output_get (Variables|Default|SetActiveLauncher _outitem))
          (Default|LaunchToy _output_get)
          (else
            (CallFunction|FireRandomLauncher)))))))