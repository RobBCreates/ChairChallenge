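; BP_Snowman is an interactable snowman in the Snow Toss challenge that opens a dialogue with the player.
; The interact pop-up functions forward to the GMCInteractable component, and showing the pop-up enables interaction.
; Interacting creates the dialogue box widget, hides the player pawn and switches the view to the snowman.
; It also locks player movement and actions, focuses mouse input on the widget and disables further interaction.
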(event EventBeginPlay)

(event Collision|EventActorBeginOverlap
  (params (OtherActor :type Actor%20Object%20Reference)))

(event Collision|EventActorEndOverlap
  (params (OtherActor :type Actor%20Object%20Reference)))

(fn ConstructionScript)

(fn DisplayInteractPopUp
  (params (Caller :type Actor%20Object%20Reference))
  (Class|GMCInteractableComponent|CallDisplayPopUp (Variables|Default|GetGMCInteractable))
  (bind _output_get (Variables|Default|SetCanInteract true))
  (return _output_get))

(fn HideInteractPopUp
  (params (Caller :type Actor%20Object%20Reference))
  (Class|GMCInteractableComponent|CallHidePopUp (Variables|Default|GetGMCInteractable))
  (return false))

(fn Interact
  (params (CallingActor :type Actor%20Object%20Reference))
  (if (Variables|Default|GetCanInteract)
    (bind _asbp_gmchero (Utilities|Casting|CastToBP_GMCHero CallingActor))
    (Variables|Default|SetGMCHero _asbp_gmchero)
    (Class|GMCInteractableComponent|CallInteract (Variables|Default|GetGMCInteractable))
    (CallFunction|HideInteractPopUp)
    (bind _asbp_gmcplayer_controller (Utilities|Casting|CastToBP_GMCPlayerController (Game|GetPlayerController 0)))
    (bind _output_get (LocalVariables|SetGMCController _asbp_gmcplayer_controller))
    (bind _returnvalue (UserInterface|CreateWidget "/Game/GMC/Challenges/Challenge_002_SnowToss/UI/WBP_002_DialogueBox.WBP_002_DialogueBox_C" _output_get))
    (bind _output_get_2 (Variables|Default|SetDialogueWidget _returnvalue))
    (UserInterface|Viewport|AddtoViewport _output_get_2 0)
    (Rendering|SetActorHiddenInGame (Game|Player|GetPlayerPawn 0) true)
    (Game|Player|SetViewTargetwithBlend (LocalVariables|GetGMCController) self 0.0 "VTBlend_Linear" 0.0 false)
    (Class|GMCPlayerController|LockPlayerMovement (LocalVariables|GetGMCController) true)
    (Class|GMCPlayerController|LockPlayerActions (LocalVariables|GetGMCController) true)
    (Variables|/Script/Engine.PlayerController|SetbShowMouseCursor (LocalVariables|GetGMCController) true)
    (Input|SetInputModeGameandUI (LocalVariables|GetGMCController) (Variables|Default|GetDialogueWidget) "DoNotLock" true)
    (Variables|Default|SetCanInteract false)
    (return self)))