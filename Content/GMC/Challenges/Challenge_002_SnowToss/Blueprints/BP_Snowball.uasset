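; BP_Snowball is a throwable snowball projectile for the SnowToss challenge.
; Toss sets the ProjectileMovement velocity along a given forward vector, activates it, and has the mesh ignore the instigator while moving.
; A hit or a projectile stop plays the snowball impact sound at its location and destroys the actor.
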(event OnProjectileStop(ProjectileMovement)
  (params (ImpactResult :type Hit%20Result%20Structure%20%28by%20ref%29))
  (Audio|PlaySoundatLocation "/Game/GMC/Challenges/Challenge_002_SnowToss/Audio/SFX/SnowballHit.SnowballHit" (Transformation|GetActorLocation) "0, 0, 0" 1.0 1.0 0.0 0 0 0)
  (Actor|DestroyActor))

(event Custom|OnHit
  (Audio|PlaySoundatLocation "/Game/GMC/Challenges/Challenge_002_SnowToss/Audio/SFX/SnowballHit.SnowballHit" (Transformation|GetActorLocation) "0, 0, 0" 1.0 1.0 0.0 0 0 0)
  (Actor|DestroyActor))

(event Custom|Toss
  (params (ForwardVector :type Vector))
  (Variables|/Script/Engine.MovementComponent|SetVelocity (Variables|Default|GetProjectileMovement) (* ForwardVector 1.5e+03))
  (Components|Activation|Activate (Variables|Default|GetProjectileMovement) false)
  (Collision|IgnoreActorwhenMoving (Variables|Debug|GetStaticMeshComponent) (Game|GetInstigator) true))

(event EventBeginPlay)

(event Collision|EventActorBeginOverlap
  (params (OtherActor :type Actor%20Object%20Reference)))

(event EventTick
  (params (DeltaSeconds :type Float%20%28single-precision%29)))

(fn ConstructionScript)