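; Gallery character that displays a configurable sitting pose through its BPSitComp component.
; The construction script copies its pose number, sit state, sit type and mirror settings into the component.
; Shortly after BeginPlay it switches the component's sit state.
; Tick clears the turn flag through a short delay and clamps the pose number using a per-sit-type Select whose index is fixed to Chair.
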(event EventTick
  (params (DeltaSeconds :type Float%20%28single-precision%29))
  (bind _bp_sitcomp (Variables|Default|GetBP_SitComp))
  (Utilities|FlowControl|Sequence
    (:then_0
      (Utilities|FlowControl|Delay 0.01)
      (Variables|/Game/SittingAnimations/Blueprints/BP_SitComp.BP_SitComp_C|SetTurn (Variables|Default|GetBP_SitComp) false))
    (:then_1
      (Variables|/Game/SittingAnimations/Blueprints/BP_SitComp.BP_SitComp_C|SetPoseNumber _bp_sitcomp (Math|Integer|Clamp(Integer) (Variables|/Game/SittingAnimations/Blueprints/BP_SitComp.BP_SitComp_C|GetPoseNumber _bp_sitcomp) 0 (Utilities|Select :Index "NewEnumerator0" :NewEnumerator0 14 :NewEnumerator1 11 :NewEnumerator2 4))))))

(event EventBeginPlay
  (Utilities|FlowControl|Delay 1.0)
  (Variables|/Game/SittingAnimations/Blueprints/BP_SitComp.BP_SitComp_C|SetSitStates (Variables|Default|GetBP_SitComp) "NewEnumerator2"))

(fn ConstructionScript
  (bind _bp_sitcomp (Variables|Default|GetBP_SitComp))
  (Variables|/Game/SittingAnimations/Blueprints/BP_SitComp.BP_SitComp_C|SetPoseNumber _bp_sitcomp (Variables|Default|GetPoseNumber))
  (Variables|/Game/SittingAnimations/Blueprints/BP_SitComp.BP_SitComp_C|SetSitStates _bp_sitcomp (Variables|Default|GetSitStates))
  (Variables|/Game/SittingAnimations/Blueprints/BP_SitComp.BP_SitComp_C|SetSitType _bp_sitcomp (Variables|Default|GetSitType))
  (Variables|/Game/SittingAnimations/Blueprints/BP_SitComp.BP_SitComp_C|SetMirror _bp_sitcomp (Variables|Default|GetMirror)))